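; BP_GameManager watches for the end of a round by counting living BP_FirstPersonCharacter actors and showing a win screen.
; After a short delay from BeginPlay, a fast looping timer recounts all characters not flagged IsDead.
; When at most one remains, it adds WBP_WinScreen to the viewport and enables the mouse cursor for player 0.
; The timer is never cleared, so the widget can be created repeatedly.
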(event Custom|CheckPlayers
  (Variables|Default|SetAlivePlayers 0)
  (bind _outactors (Actor|GetAllActorsOfClass "/Game/FirstPerson/Blueprints/BP_FirstPersonCharacter.BP_FirstPersonCharacter_C"))
  (for _array_element _outactors
    (if (not (Variables|/Game/FirstPerson/Blueprints/BP_FirstPersonCharacter.BP_FirstPersonCharacter_C|GetIsDead _array_element))
      (bind _result (Math|Integer|IncrementInt (Variables|Default|GetAlivePlayers)))))
  (if (<= _result 1)
    (bind _returnvalue (UserInterface|CreateWidget "/Game/UI/WBP_WinScreen.WBP_WinScreen_C"))
    (UserInterface|Viewport|AddtoViewport _returnvalue 0)
    (Variables|/Script/Engine.PlayerController|SetbShowMouseCursor (Game|GetPlayerController (Variables|/Script/Engine.Pawn|GetPlayerState (Game|GetPlayerCharacter 0))) true)))

(event EventBeginPlay
  (Utilities|FlowControl|Delay 1.0)
  (Utilities|Time|SetTimerbyEvent (delegate Custom|CheckPlayers) 0.2 true))

(fn ConstructionScript)