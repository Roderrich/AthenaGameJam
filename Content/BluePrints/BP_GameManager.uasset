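; Game manager Blueprint that detects when at most one player is left alive and shows the win screen.
; After a one-second delay at BeginPlay, a looping timer counts living BP_FirstPersonCharacter actors.
; At one or none, it creates WBP_WinScreen with LastPlayer and shows player 0's cursor.
; The timer is never cleared, and LastPlayer is only assigned to itself.
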(event Custom|CheckPlayers
  (Variables|Default|SetAlivePlayers 0)
  (bind _outactors (Actor|GetAllActorsOfClass "/Game/BluePrints/BP_FirstPersonCharacter.BP_FirstPersonCharacter_C"))
  (bind _output_get (Variables|Default|SetOut%20Actors _outactors))
  (for _array_element _output_get
    (if (not (Variables|/Game/BluePrints/BP_FirstPersonCharacter.BP_FirstPersonCharacter_C|GetIsDead _array_element))
      (bind _result (Math|Integer|IncrementInt (Variables|Default|GetAlivePlayers))
        (:%20%20
          (bind _output_get_2 (Variables|Default|SetLastPlayer (Variables|Default|GetLastPlayer)))))))
  (if (<= _result 1)
    (bind _returnvalue (UserInterface|CreateWidget "/Game/UI/WBP_WinScreen.WBP_WinScreen_C" 0 _output_get_2))
    (UserInterface|Viewport|AddtoViewport _returnvalue 0)
    (Variables|/Script/Engine.PlayerController|SetbShowMouseCursor (Game|GetPlayerController (Variables|/Script/Engine.Pawn|GetPlayerState (Game|GetPlayerCharacter 0))) true)))

(event EventBeginPlay
  (Utilities|FlowControl|Delay 1.0)
  (Utilities|Time|SetTimerbyEvent (delegate Custom|CheckPlayers) 0.2 true))

(fn ConstructionScript)