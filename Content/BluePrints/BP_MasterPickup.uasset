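; Pickup actor that grants one of seven power-ups (elemental cooldown, damage, range or speed) to BP_FirstPersonCharacter.
; The construction script randomly picks the type and sets the matching billboard sprite, which two timelines bob and yaw during play.
; On overlap it passes the type to the character's ManagePickups, hides, disables collision, plays a type-specific sound and destroys itself after a delay.
; Any damage destroys it immediately.
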(event OnComponentBeginOverlap(box_0)
  (params (OverlappedComponent :type Primitive%20Component%20Object%20Reference) (OtherActor :type Actor%20Object%20Reference) (OtherComp :type Primitive%20Component%20Object%20Reference) (OtherBodyIndex :type Integer) (bFromSweep :type Boolean) (SweepResult :type Hit%20Result%20Structure%20%28by%20ref%29))
  (bind _audio1 (Variables|Default|GetAudio1))
  (bind _asbp_first_person_character (Utilities|Casting|CastToBP_FirstPersonCharacter OtherActor))
  (Default|ManagePickups _asbp_first_person_character (Variables|Default|GetPickUpType))
  (Rendering|SetVisibility (Variables|Default|GetDefaultSceneRoot) false true)
  (Collision|SetCollisionEnabled (Variables|Default|Getbox_0) "NoCollision")
  (switch string (Variables|Default|GetPickUpType)
    (:EarthCD
      (Audio|Components|Audio|SetSound _audio1 "/Game/Sounds/PickUpSounds/earth_cool_down_Cue.earth_cool_down_Cue"))
    (:FireCD
      (Audio|Components|Audio|SetSound _audio1 "/Game/Sounds/PickUpSounds/fire_cool_down_Cue.fire_cool_down_Cue"))
    (:IceCD
      (Audio|Components|Audio|SetSound _audio1 "/Game/Sounds/PickUpSounds/ice_cool_down_Cue.ice_cool_down_Cue"))
    (:FireDmg
      (Audio|Components|Audio|SetSound _audio1 "/Game/Sounds/PickUpSounds/fire_damage_Cue.fire_damage_Cue"))
    (:IceDmg
      (Audio|Components|Audio|SetSound _audio1 "/Game/Sounds/PickUpSounds/ice_damage_Cue.ice_damage_Cue"))
    (:SpeedUp
      (Audio|Components|Audio|SetSound _audio1 "/Game/Sounds/PickUpSounds/speed_boost_Cue.speed_boost_Cue"))
    (:FireRange
      (Audio|Components|Audio|SetSound _audio1 "/Game/Sounds/PickUpSounds/fire_range_Cue.fire_range_Cue")))
  (Audio|Components|Audio|Play _audio1 0.0)
  (Utilities|FlowControl|Delay 5.0)
  (Actor|DestroyActor))

(event EventBeginPlay
  (bind _billboard (Variables|Default|GetBillboard))
  (bind _returnvalue (Transformation|GetWorldRotation _billboard))
  (bind _output_get (Variables|Default|SetStartVector (.location (Transformation|GetWorldTransform (Variables|Default|GetBillboard)))))
  (bind _newtrack_0 (Timeline|Timeline Play)
    (:Update
      (bind _newtrack_0_2 (Timeline|Timeline_0 Play)
        (:Update
          (Transformation|SetWorldLocationAndRotation (Variables|Default|GetBillboard) (+ _output_get (Math|Vector|MakeVector 0.0 0.0 _newtrack_0)) (Math|Rotator|MakeRotator (.roll _returnvalue) (.pitch _returnvalue) _newtrack_0_2) false false))))))

(event Game|Damage|EventAnyDamage
  (params (Damage :type Float%20%28single-precision%29) (DamageType :type Damage%20Type%20Object%20Reference) (InstigatedBy :type Controller%20Object%20Reference) (DamageCauser :type Actor%20Object%20Reference))
  (Actor|DestroyActor))

(fn ConstructionScript
  (bind _billboard (Variables|Default|GetBillboard))
  (switch Utilities|FlowControl|Switch|SwitchonPickUpTypes (Utilities|Enum|ByteToEnumPickUpTypes (Math|Conversions|ToByte(Integer) (Math|Random|RandomIntegerinRange 0 (- (|GetNumEnumEntries) 1))))
    (:NewEnumerator0
      (Variables|Default|SetPickUpType "EarthCD")
      (Rendering|Components|Sprite|SetSprite _billboard "/Game/Powerup_Sprites/Earth_cooldown.Earth_cooldown"))
    (:NewEnumerator1
      (Variables|Default|SetPickUpType "FireCD")
      (Rendering|Components|Sprite|SetSprite _billboard "/Game/Powerup_Sprites/Fire_cooldown.Fire_cooldown"))
    (:NewEnumerator2
      (Variables|Default|SetPickUpType "IceCD")
      (Rendering|Components|Sprite|SetSprite _billboard "/Game/Powerup_Sprites/Ice_cooldown.Ice_cooldown"))
    (:NewEnumerator3
      (Variables|Default|SetPickUpType "FireDmg")
      (Rendering|Components|Sprite|SetSprite _billboard "/Game/Powerup_Sprites/Fire_damage.Fire_damage"))
    (:NewEnumerator4
      (Variables|Default|SetPickUpType "IceDmg")
      (Rendering|Components|Sprite|SetSprite _billboard "/Game/Powerup_Sprites/Ice_damage.Ice_damage"))
    (:NewEnumerator5
      (Variables|Default|SetPickUpType "SpeedUp")
      (Rendering|Components|Sprite|SetSprite _billboard "/Game/Powerup_Sprites/Speed_boost.Speed_boost"))
    (:NewEnumerator6
      (Variables|Default|SetPickUpType "FireRange")
      (Rendering|Components|Sprite|SetSprite _billboard "/Game/Powerup_Sprites/Range_powerup.Range_powerup"))))