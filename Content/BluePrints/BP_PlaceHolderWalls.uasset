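; BP_PlaceHolderWalls is a placeholder actor that marks where an earth wall and a possible pickup spawn.
; On BeginPlay it spawns BP_Earth_Def_01 at its root's world transform, unless the FirstSpawn flag is set.
; A separate CreateItem event has a one-in-two chance to spawn BP_MasterPickup slightly above the root, with the same rotation.
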(event Custom|CreateItem
  (bind _defaultsceneroot (Variables|Default|GetDefaultSceneRoot))
  (bind _returnvalue (Transformation|GetWorldTransform _defaultsceneroot))
  (if (== (Math|Random|RandomIntegerinRange 0 1) 0)
    (Game|SpawnActorfromClass "/Game/Pickups/BP_MasterPickup.BP_MasterPickup_C" (Math|Transform|MakeTransform (+ (.location _returnvalue) "0.000000,0.000000,100.000000") (.rotation _returnvalue) "1.000000,1.000000,1.000000") "Undefined" "MultiplyWithRoot" 0 0)))

(event EventBeginPlay
  (bind _defaultsceneroot (Variables|Default|GetDefaultSceneRoot))
  (bind _returnvalue (Transformation|GetWorldTransform _defaultsceneroot))
  (if (not (Variables|Default|GetFirstSpawn))
    (Game|SpawnActorfromClass "/Game/Luos8Elements/Blueprints/Earth/BP_Earth_Def_01.BP_Earth_Def_01_C" (Math|Transform|MakeTransform (Math|Vector|MakeVector (.x (.location _returnvalue)) (.y (.location _returnvalue)) (.z (.location _returnvalue))) (.rotation _returnvalue) (.scale _returnvalue)) "Undefined" "MultiplyWithRoot" 0 0)))

(fn ConstructionScript)