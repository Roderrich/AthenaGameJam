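; Health component that tracks an integer Heath value and mirrors changes to heart displays in the Main_ui widget.
; ModifyHeath adds a signed amount clamped between zero and MaxHeath, then calls UpdateHearts one step at a time for each point of the requested, unclamped amount.
; The widget is looked up by class on every step, and reaching zero only prints a red "dead" debug message inside that loop.
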(event EventBeginPlay)

(fn ModifyHeath
  (params (Heath%20Amount :type Integer))
  (Variables|Default|SetHeath (Math|Integer|Clamp(Integer) (+ Heath%20Amount (Variables|Default|GetHeath)) 0 (Variables|Default|GetMaxHeath)))
  (for _index (range 1 (Math|Integer|Absolute(Integer) Heath%20Amount))
    (bind _foundwidgets (Widget|GetAllWidgetsOfClass "/Game/UI/Main_ui.Main_ui_C" true))
    (Default|UpdateHearts (Utilities|Array|Get(acopy) _foundwidgets) (select (> Heath%20Amount 0) 1 -1))
    (if (<= (Variables|Default|GetHeath) 0)
      (Development|PrintString "dead" true true "(R=1.000000,G=0.000000,B=0.000000,A=1.000000)"))))