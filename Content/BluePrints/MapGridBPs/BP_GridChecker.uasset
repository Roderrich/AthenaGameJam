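; BP_GridChecker is a moving probe that spreads an explosion along the map grid toward a target location.
; A timeline on BeginPlay lerps it from its current position to the target, destroying it on arrival or once inactive.
; Its sphere overlaps explode and damage grid sections.
; Pillars and placeholder walls halt it; with a valid last section, a wall also re-damages that section, spawns an item, plays audio and is destroyed.
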(event OnComponentBeginOverlap(Sphere)
  (params (OverlappedComponent :type Primitive%20Component%20Object%20Reference) (OtherActor :type Actor%20Object%20Reference) (OtherComp :type Primitive%20Component%20Object%20Reference) (OtherBodyIndex :type Integer) (bFromSweep :type Boolean) (SweepResult :type Hit%20Result%20Structure%20%28by%20ref%29))
  (bind _firedamage (Variables|Default|GetFireDamage))
  (bind _ownerplayer (Variables|Default|GetOwnerPlayer))
  (bind _asbp_grid_section (Utilities|Casting|CastToBP_GridSection OtherActor)
    (:then
      (bind _output_get (Variables|Default|SetLastGrid _asbp_grid_section))
      (if (stale _output_get_2)
        (Default|ExplodeThisGrid _output_get)
        (Default|DamagePlayer _output_get _firedamage _ownerplayer)))
    (:CastFailed
      (bind _asbp_place_holder_walls (Utilities|Casting|CastToBP_PlaceHolderWalls OtherActor)
        (:then
          (bind _output_get_2 (Variables|Default|SetisActive false))
          (Utilities|IsValid _output_get
            (:Is%20Valid
              (Default|DamagePlayer _output_get _firedamage _ownerplayer)
              (Default|CreateItem _asbp_place_holder_walls)
              (Audio|Components|Audio|Play (Variables|Default|GetAudio) 0.0)
              (Actor|DestroyActor _asbp_place_holder_walls)
              (Components|DestroyComponent (Variables|Default|GetSphere)))))
        (:CastFailed
          (Utilities|Casting|CastToBP_Pillar OtherActor)
          (Variables|Default|SetisActive false)
          (Components|DestroyComponent (Variables|Default|GetSphere)))))))

(event EventBeginPlay
  (bind _defaultsceneroot (Variables|Default|GetDefaultSceneRoot))
  (bind _returnvalue (Transformation|GetWorldLocation _defaultsceneroot))
  (bind _alpha (Timeline|Alpha Play)
    (:Update
      (if (stale OnComponentBeginOverlap(Sphere) _output_get_2)
        (Transformation|SetWorldLocation _defaultsceneroot (Math|Vector|Lerp(Vector) _returnvalue (Variables|Default|GetTarget%20Relative%20Location) _alpha) false false)
        (if (Utilities|Operators|EqualEqual _returnvalue (Variables|Default|GetTarget%20Relative%20Location) 1.0)
          (Actor|DestroyActor :!label _label))
        (else
          (goto _label))))))

(fn ConstructionScript)