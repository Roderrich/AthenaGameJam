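; Earth defense spell effect actor that plays a short-lived set of five earth magic particle systems.
; On BeginPlay it activates all particle components, then after a brief delay plays a timeline.
; A timeline event deactivates every particle and destroys the actor, so the effect cleans itself up.
; It contains no gameplay logic such as collision, damage or blocking.
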(event EventBeginPlay
  ;[1 1 1] 1. Activates particle
  (Components|Activation|Activate (Variables|Default|GetPar_LMagic_Earth_Def_01a) false)
  (Utilities|FlowControl|Delay 0.2)
  ;[1 1 1] Deactivate_Particles
  (Timeline|TL_Earth_Def Play
    (:DeActivate%20All
      ;[1 1 1] Deactivates Particle.
      (Components|Activation|Deactivate (Variables|Default|GetPar_LMagic_Earth_Def_01a))
      (Actor|DestroyActor))))

(event Collision|EventActorBeginOverlap
  (params (OtherActor :type Actor%20Object%20Reference)))

(event EventTick
  (params (DeltaSeconds :type Float%20%28single-precision%29)))

(fn ConstructionScript)