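; BP_Fire_Atk_01 is a fire attack spell actor that tracks which grid section it occupies.
; One tick after BeginPlay, it stores the first grid section overlapping its sphere as the initial location, recording it as last valid if not wall-overlapped.
; Each later grid overlap updates the current and last locations, except wall-overlapped sections, which set current back to the last valid section.
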(event Collision|EventActorBeginOverlap
  (params (OtherActor :type Actor%20Object%20Reference))
  (bind _asbp_grid_section (Utilities|Casting|CastToBP_GridSection OtherActor))
  (if (Variables|/Game/BluePrints/MapGridBPs/BP_GridSection.BP_GridSection_C|GetisOverlappedWall _asbp_grid_section)
    (Variables|Default|SetCurrentGridLocation (Variables|Default|GetLastGridLocation))
    (else
      (bind _output_get (Variables|Default|SetCurrentGridLocation _asbp_grid_section))
      (Variables|Default|SetLastGridLocation _output_get))))

(event EventBeginPlay
  (bind _sphere (Variables|Default|GetSphere))
  (bind _overlappingactors (Collision|GetOverlappingActors _sphere "/Game/BluePrints/MapGridBPs/BP_GridSection.BP_GridSection_C" :!class /Script/Engine.PrimitiveComponent))
  (Utilities|FlowControl|DelayUntilNextTick)
  (if (not (Utilities|Array|IsEmpty _overlappingactors))
    (bind _output_get (Variables|Default|SetInitialGridLocation (Utilities|Array|Get(acopy) _overlappingactors)))
    (Utilities|IsValid _output_get
      (:Is%20Valid
        (bind _asbp_grid_section (Utilities|Casting|CastToBP_GridSection _output_get))
        (if (not (Variables|/Game/BluePrints/MapGridBPs/BP_GridSection.BP_GridSection_C|GetisOverlappedWall _asbp_grid_section))
          (Variables|Default|SetLastGridLocation _asbp_grid_section))))))

(fn ConstructionScript
  (|CallParentFunction))