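; Fire attack actor from the 8 Elements set that tracks which BP_GridSection it occupies.
; On BeginPlay it stores the first grid section overlapping its Sphere as the last location.
; Each new section overlap becomes both current and last location, unless that section is flagged IsOverlapped, in which case the current location reverts to the last one.
; The graph holds only this grid tracking, with no damage or movement logic.
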(event Collision|EventActorBeginOverlap
  (params (OtherActor :type Actor%20Object%20Reference))
  (bind _asbp_grid_section (Utilities|Casting|CastToBP_GridSection OtherActor))
  (if (Variables|/Game/Map_Grid/BP_GridSection.BP_GridSection_C|GetisOverlapped _asbp_grid_section)
    (Variables|Default|SetCurrentGridLocation (Variables|Default|GetLastGridLocation))
    (else
      (bind _output_get (Variables|Default|SetCurrentGridLocation _asbp_grid_section))
      (Variables|Default|SetLastGridLocation _output_get))))

(event EventBeginPlay
  (bind _sphere (Variables|Default|GetSphere))
  (bind _overlappingactors (Collision|GetOverlappingActors _sphere "/Game/Map_Grid/BP_GridSection.BP_GridSection_C" :!class /Script/Engine.PrimitiveComponent))
  (if (not (Utilities|Array|IsEmpty _overlappingactors))
    (bind _asbp_grid_section (Utilities|Casting|CastToBP_GridSection (Utilities|Array|Get(acopy) _overlappingactors)))
    (Variables|Default|SetLastGridLocation _asbp_grid_section)))

(fn ConstructionScript
  (|CallParentFunction))