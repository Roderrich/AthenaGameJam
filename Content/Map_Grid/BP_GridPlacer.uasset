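; BP_GridPlacer generates a 3D grid of BP_GridSection actors from its location and fills the bottom layer with placeholder walls.
; On BeginPlay it spawns sections sized by GridScale, then after a short delay runs FillGrid.
; FillGrid walks the first layer, skipping EmptyInts indices and overlapped sections, and spawns BP_PlaceHolderWalls at each cube's base.
; BuildGrid and ClearGrid events rebuild or destroy the tracked sections and walls.
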(event Custom|BuildGrid
  (CallFunction|CreateGridFunc)
  (CallFunction|FillGrid))

(event Custom|ClearGrid
  (CallFunction|ClearGridFunc)
  (CallFunction|ClearFilledGrid))

(event EventBeginPlay
  (CallFunction|CreateGridFunc)
  (Utilities|FlowControl|Delay 1.0)
  (CallFunction|FillGrid))

(fn ConstructionScript)

(fn ClearGridFunc
  (for _array_element (Variables|Default|GetGridSectionArray)
    (Actor|DestroyActor _array_element)))

(fn CreateGridFunc
  (bind _width (Variables|Default|GetWidth))
  (bind _depth (Variables|Default|GetDepth))
  (bind _gridscale (Variables|Default|GetGridScale))
  (bind _basegridscale (LocalVariables|GetBaseGridScale))
  (bind _gridscale_2 (Variables|Default|GetGridScale))
  (bind _gridheight (LocalVariables|GetGridHeight))
  (bind _gridscale_3 (Variables|Default|GetGridScale))
  (bind _gridscale_4 (Variables|Default|GetGridScale))
  (bind _returnvalue (* _basegridscale _gridscale_4))
  (bind _returnvalue_2 (* _gridheight _gridscale_3))
  (bind _returnvalue_3 (/ _width _gridscale))
  (bind _returnvalue_4 (/ _depth _gridscale_2))
  (Variables|Default|SetArrayInt 0)
  (Variables|Default|SetTransformOffest (Transformation|GetWorldLocation (Variables|Default|GetDefaultSceneRoot)))
  (Variables|Default|SetFirstLayerInt (* _returnvalue_4 _returnvalue_3))
  (for _index (range 0 (- (/ (Variables|Default|GetHeight) (Variables|Default|GetGridScale)) 1))
    (for _index_2 (range 0 (- _returnvalue_3 1))
      (for _index_3 (range 0 (- _returnvalue_4 1))
        (bind _returnvalue_5 (Game|SpawnActorfromClass "/Game/Map_Grid/BP_GridSection.BP_GridSection_C" (Math|Transform|MakeTransform (+ (Math|Vector|MakeVector (Math|Conversions|ToFloat(Integer) (* _index_2 _returnvalue)) (Math|Conversions|ToFloat(Integer) (* _index_3 _returnvalue)) (Math|Conversions|ToFloat(Integer) (* _index _returnvalue))) (Math|Vector|MakeVector (+ (.x (Variables|Default|GetTransformOffest)) _returnvalue_2) (+ (.y (Variables|Default|GetTransformOffest)) _returnvalue_2) _returnvalue_2)) "0, 0, 0" (* (LocalVariables|GetBaseVectorScale) (Variables|Default|GetGridScale))) "Undefined" "MultiplyWithRoot" 0 (Variables|Default|GetisDebug) (Math|Vector|MakeVector (Math|Conversions|ToFloat(Integer) _index_2) (Math|Conversions|ToFloat(Integer) _index_3) (Math|Conversions|ToFloat(Integer) _index)) (Variables|Default|GetArrayInt) (Variables|Default|GetGridScale) 0))
        (Utilities|Array|Add (Variables|Default|GetGridSectionArray) _returnvalue_5)
        (Math|Integer|IncrementInt (Variables|Default|GetArrayInt))))))

(fn FillGrid
  (bind (_array_element _array_index) (Utilities|Array|ForEachLoopwithBreak (Variables|Default|GetGridSectionArray) :!label _label)
    (:LoopBody
      (if (< _array_index (Variables|Default|GetFirstLayerInt))
        (if (== _array_index (Utilities|Array|Get(acopy) (Variables|Default|GetEmptyInts) (Variables|Default|Getcurrentemptyindex)))
          (Math|Integer|IncrementInt (Variables|Default|Getcurrentemptyindex))
          (elif (not (Variables|/Game/Map_Grid/BP_GridSection.BP_GridSection_C|GetisOverlapped _array_element))
            (bind _returnvalue (Game|SpawnActorfromClass "/Game/BP_PlaceHolderWalls.BP_PlaceHolderWalls_C" (Math|Transform|MakeTransform (Transformation|GetWorldLocation (Variables|/Game/Map_Grid/BP_GridSection.BP_GridSection_C|GetBase%20of%20cube _array_element)) "0, 0, 0" (* (Variables|Default|GetGridScale) (LocalVariables|GetNewLocalVar))) "Undefined" "MultiplyWithRoot" 0 true 0))
            (Utilities|Array|Add (Variables|Default|GetPlacedWallsArray) _returnvalue)))
        (else
          (goto _label Break))))))

(fn ClearFilledGrid
  (for _array_element (Variables|Default|GetPlacedWallsArray)
    (Actor|DestroyActor _array_element)))