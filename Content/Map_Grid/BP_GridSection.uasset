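; BP_GridSection is one map grid cell that tracks occupancy and reacts to spells.
; Box overlaps and a looping timer update occupancy by players, walls and pillars, with a debug cube display; other actors set a projectile flag.
; Fire hits send BP_GridCheckers toward five level-scaled axis points (no downward one), while Earth hits spawn a wall.
; Separate events spawn fire on the cell and deal flat damage to overlapping players, ignoring Level.
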(event OnComponentBeginOverlap(Box)
  (params (OverlappedComponent :type Primitive%20Component%20Object%20Reference) (OtherActor :type Actor%20Object%20Reference) (OtherComp :type Primitive%20Component%20Object%20Reference) (OtherBodyIndex :type Integer) (bFromSweep :type Boolean) (SweepResult :type Hit%20Result%20Structure%20%28by%20ref%29))
  (Utilities|Casting|CastToBP_FirstPersonCharacter OtherActor
    (:then
      (Variables|Default|SetisOverlapped true :!label _label)
      (if (Variables|Default|GetisDebug)
        (Rendering|SetVisibility (Variables|Default|GetCube) true false)))
    (:CastFailed
      (Utilities|Casting|CastToBP_PlaceHolderWalls OtherActor
        (:then
          (goto _label))
        (:CastFailed
          (Utilities|Casting|CastToBP_Pillar OtherActor
            (:then
              (goto _label))
            (:CastFailed
              (Variables|Default|SetisOverlappedByProjectile true))))))))

(event OnComponentEndOverlap(Box)
  (params (OverlappedComponent :type Primitive%20Component%20Object%20Reference) (OtherActor :type Actor%20Object%20Reference) (OtherComp :type Primitive%20Component%20Object%20Reference) (OtherBodyIndex :type Integer))
  (bind _cube (Variables|Default|GetCube))
  (bind _isdebug (Variables|Default|GetisDebug))
  (Utilities|Casting|CastToBP_FirstPersonCharacter OtherActor
    (:then
      (if (Math|Boolean|ORBoolean (> (Utilities|Array|Length (Collision|GetOverlappingActors (Variables|Default|GetBox) "/Game/BP_PlaceHolderWalls.BP_PlaceHolderWalls_C" :!class /Script/Engine.PrimitiveComponent)) 0) (> (Utilities|Array|Length (Collision|GetOverlappingActors (Variables|Default|GetBox) "/Game/FirstPerson/Blueprints/BP_FirstPersonCharacter.BP_FirstPersonCharacter_C" :!class /Script/Engine.PrimitiveComponent)) 0) (> (Utilities|Array|Length (Collision|GetOverlappingActors (Variables|Default|GetBox) "/Game/BP_Pillar.BP_Pillar_C" :!class /Script/Engine.PrimitiveComponent)) 0)) :!label _label
        (Variables|Default|SetisOverlapped true)
        (if _isdebug
          (Rendering|SetVisibility _cube true false))
        (else
          (Variables|Default|SetisOverlapped false)
          (if _isdebug
            (Rendering|SetVisibility _cube false false)))))
    (:CastFailed
      (Utilities|Casting|CastToBP_PlaceHolderWalls OtherActor
        (:then
          (goto _label))
        (:CastFailed
          (Variables|Default|SetisOverlappedByProjectile false))))))

(event Custom|SpellHitGrid
  (params (Type :type SpellsEnum%20Enum :default "NewEnumerator0") (Level :type Integer) (OwnerPlayer :type BP%20First%20Person%20Character%20Object%20Reference))
  (bind _cube (Variables|Default|GetCube))
  (switch Utilities|FlowControl|Switch|SwitchonSpellsEnum Type
    (:NewEnumerator0
      (CallFunction|ExplosionNeighbourstoCheck Level)
      (CallFunction|CreateGridCheckers (Transformation|GetWorldLocation _cube) (Transformation|GetWorldRotation _cube) Level OwnerPlayer))
    (:NewEnumerator2
      (CallFunction|CreateWall))))

(event Custom|CheckEmpty
  (bind _cube (Variables|Default|GetCube))
  (bind _isdebug (Variables|Default|GetisDebug))
  (if (Math|Boolean|ORBoolean (> (Utilities|Array|Length (Collision|GetOverlappingActors (Variables|Default|GetBox) "/Game/BP_PlaceHolderWalls.BP_PlaceHolderWalls_C" :!class /Script/Engine.PrimitiveComponent)) 0) (> (Utilities|Array|Length (Collision|GetOverlappingActors (Variables|Default|GetBox) "/Game/FirstPerson/Blueprints/BP_FirstPersonCharacter.BP_FirstPersonCharacter_C" :!class /Script/Engine.PrimitiveComponent)) 0) (> (Utilities|Array|Length (Collision|GetOverlappingActors (Variables|Default|GetBox) "/Game/BP_Pillar.BP_Pillar_C" :!class /Script/Engine.PrimitiveComponent)) 0))
    (Variables|Default|SetisOverlapped true)
    (if _isdebug
      (Rendering|SetVisibility _cube true false))
    (else
      (Variables|Default|SetisOverlapped false)
      (if _isdebug
        (Rendering|SetVisibility _cube false false)))))

(event Custom|ExplodeThisGrid
  (bind _gridscale (Variables|Default|GetGridScale))
  (bind _base_of_cube (Variables|Default|GetBase%20of%20cube))
  (Game|SpawnActorfromClass "/Game/Luos8Elements/Blueprints/Fire/BP_Fire_Grid.BP_Fire_Grid_C" (Math|Transform|MakeTransform (+ (Transformation|GetWorldLocation _base_of_cube) (* _gridscale (Variables|Default|GetFireVec))) (Transformation|GetWorldRotation _base_of_cube) (* _gridscale (Variables|Default|GetFireVecScale))) "Undefined" "MultiplyWithRoot" 0 0))

(event Custom|DamagePlayer
  (params (level :type Integer) (OwnerPlayer :type BP%20First%20Person%20Character%20Object%20Reference))
  (for _array_element (Collision|GetOverlappingActors (Variables|Default|GetBox) "/Game/FirstPerson/Blueprints/BP_FirstPersonCharacter.BP_FirstPersonCharacter_C" :!class /Script/Engine.PrimitiveComponent)
    (bind _asbp_first_person_character (Utilities|Casting|CastToBP_FirstPersonCharacter _array_element))
    (Game|Damage|ApplyDamage _asbp_first_person_character 1.0 0 OwnerPlayer)))

(event Custom|CheckOverlapped
  (Development|PrintString (Utilities|String|Append "Number of players overlapping this grid is" (Utilities|String|ToString(Integer) (Utilities|Array|Length (Collision|GetOverlappingActors (Variables|Default|GetBox) "/Game/FirstPerson/Blueprints/BP_FirstPersonCharacter.BP_FirstPersonCharacter_C" :!class /Script/Engine.PrimitiveComponent)))))
  (Development|PrintString (Utilities|String|Append "Number of Walls overlapping this grid is" (Utilities|String|ToString(Integer) (Utilities|Array|Length (Collision|GetOverlappingActors (Variables|Default|GetBox) "/Game/BP_PlaceHolderWalls.BP_PlaceHolderWalls_C" :!class /Script/Engine.PrimitiveComponent))))))

(event EventBeginPlay
  (Utilities|Time|SetTimerbyEvent (delegate Custom|CheckEmpty) 0.1 true))

(fn ConstructionScript)

(fn ExplosionNeighbourstoCheck
  (params (Level :type Integer))
  (bind _cube (Variables|Default|GetCube))
  (bind _returnvalue (Transformation|GetWorldLocation _cube))
  (if (< Level 1)
    (LocalVariables|SetLevelMultiplyer 1)
    (else
      (LocalVariables|SetLevelMultiplyer Level)))
  (Variables|Default|SetCardianlDirections (Utilities|Array|MakeArray (Math|Vector|MakeVector (.x _returnvalue) (.y _returnvalue) (+ (.z _returnvalue) (* (LocalVariables|GetDistanceToNextGrid) (LocalVariables|GetLevelMultiplyer)))) (Math|Vector|MakeVector (+ (.x _returnvalue) (* (LocalVariables|GetDistanceToNextGrid) (LocalVariables|GetLevelMultiplyer))) (.y _returnvalue) (.z _returnvalue)) (Math|Vector|MakeVector (- (.x _returnvalue) (* (LocalVariables|GetDistanceToNextGrid) (LocalVariables|GetLevelMultiplyer))) (.y _returnvalue) (.z _returnvalue)) (Math|Vector|MakeVector (.x _returnvalue) (+ (.y _returnvalue) (* (LocalVariables|GetDistanceToNextGrid) (LocalVariables|GetLevelMultiplyer))) (.z _returnvalue)) (Math|Vector|MakeVector (.x _returnvalue) (- (.y _returnvalue) (* (LocalVariables|GetDistanceToNextGrid) (LocalVariables|GetLevelMultiplyer))) (.z _returnvalue)))))

(fn CreateGridCheckers
  (params (SpawnTransform_Location :type Vector) (SpawnTransform_Rotation :type Rotator) (Level :type Integer) (OwnerPlayer :type BP%20First%20Person%20Character%20Object%20Reference))
  (for _array_element (Variables|Default|GetCardianlDirections)
    (Game|SpawnActorfromClass "/Game/Map_Grid/BP_GridChecker.BP_GridChecker_C" (Math|Transform|MakeTransform SpawnTransform_Location SpawnTransform_Rotation "1.000000,1.000000,1.000000") "Undefined" "MultiplyWithRoot" 0 _array_element Level OwnerPlayer 0)))

(fn CreateWall
  (bind _base_of_cube (Variables|Default|GetBase%20of%20cube))
  (Game|SpawnActorfromClass "/Game/BP_PlaceHolderWalls.BP_PlaceHolderWalls_C" (Math|Transform|MakeTransform (Transformation|GetWorldLocation _base_of_cube) (Transformation|GetWorldRotation _base_of_cube) (* (Variables|Default|GetGridScale) (LocalVariables|GetNewLocalVar))) "Undefined" "MultiplyWithRoot" 0 false 0))