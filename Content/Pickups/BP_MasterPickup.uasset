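; Master pickup actor that gives the first-person character a randomly chosen cooldown, damage, speed or range power-up.
; The construction script picks a random enum entry and stores it as a pickup type, which is passed to the character's ManagePickups when it overlaps the sphere.
; Two nested timelines bob and yaw-spin the sphere from BeginPlay.
; The actor destroys itself after collection or on taking any damage.
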(event OnComponentBeginOverlap(Sphere)
  (params (OverlappedComponent :type Primitive%20Component%20Object%20Reference) (OtherActor :type Actor%20Object%20Reference) (OtherComp :type Primitive%20Component%20Object%20Reference) (OtherBodyIndex :type Integer) (bFromSweep :type Boolean) (SweepResult :type Hit%20Result%20Structure%20%28by%20ref%29))
  (bind _asbp_first_person_character (Utilities|Casting|CastToBP_FirstPersonCharacter OtherActor))
  (Default|ManagePickups _asbp_first_person_character (Variables|Default|GetPickUpType))
  (Actor|DestroyActor))

(event EventBeginPlay
  (bind _sphere (Variables|Default|GetSphere))
  (bind _returnvalue (Transformation|GetWorldRotation _sphere))
  (bind _output_get (Variables|Default|SetStartVector (.location (Transformation|GetWorldTransform (Variables|Default|GetSphere)))))
  (bind _newtrack_0 (Timeline|Timeline Play)
    (:Update
      (bind _newtrack_0_2 (Timeline|Timeline_0 Play)
        (:Update
          (Transformation|SetWorldLocationAndRotation _sphere (+ _output_get (Math|Vector|MakeVector 0.0 0.0 _newtrack_0)) (Math|Rotator|MakeRotator (.roll _returnvalue) (.pitch _returnvalue) _newtrack_0_2) false false)
          (bind _asbp_first_person_character (Utilities|Casting|CastToBP_FirstPersonCharacter (Game|GetPlayerCharacter 0)))
          (Variables|Default|SetAs%20BP%20First%20Person%20Character _asbp_first_person_character))))))

(event Game|Damage|EventAnyDamage
  (params (Damage :type Float%20%28single-precision%29) (DamageType :type Damage%20Type%20Object%20Reference) (InstigatedBy :type Controller%20Object%20Reference) (DamageCauser :type Actor%20Object%20Reference))
  (Actor|DestroyActor))

(fn ConstructionScript
  (switch Utilities|FlowControl|Switch|SwitchonPickUpTypes (Utilities|Enum|ByteToEnumPickUpTypes (Math|Conversions|ToByte(Integer) (Math|Random|RandomIntegerinRange 0 (- (|GetNumEnumEntries) 1))))
    (:NewEnumerator0
      (Variables|Default|SetPickUpType "EarthCD"))
    (:NewEnumerator1
      (Variables|Default|SetPickUpType "FireCD"))
    (:NewEnumerator2
      (Variables|Default|SetPickUpType "IceCD"))
    (:NewEnumerator3
      (Variables|Default|SetPickUpType "FireDmg"))
    (:NewEnumerator4
      (Variables|Default|SetPickUpType "IceDmg"))
    (:NewEnumerator5
      (Variables|Default|SetPickUpType "SpeedUp"))
    (:NewEnumerator6
      (Variables|Default|SetPickUpType "FireRange"))))